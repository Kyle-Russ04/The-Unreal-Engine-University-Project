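; Editor placement tool that builds a wall of stacked TV meshes along a spline.
; Slot width sets the columns, with row counts from per-column overrides, a height curve or a default.
; A seeded stream picks weighted TVSet meshes with jitter and yaw, stacking them by height into per-entry HISM previews on construction.
; BakeToEditable replaces the preview with tagged StaticMeshActors, first destroying every tagged one in the level.
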(fn ConstructionScript
  (Variables|Default|GetbBaked
    (:then)
    (:else
      (if (Variables|Workflow|GetbAutoRebuild)
        (CallFunction|BiuldPreviewHISM)))))

(fn BuildMeshCacheandSlotSize
  (bind _targetslotsize (Variables|TVContent|GetTargetSlotSize))
  (Variables|Default|SetTotalWeight 0.0)
  (Variables|Default|SetSlotSize "0, 0, 0")
  (Utilities|Map|Clear (Variables|Default|GetMeshSizeCache))
  (for _array_element (Variables|/Game/Blueprints/PDA_TVSet.PDA_TVSet_C|GetTVEntries (Variables|TVcontent|GetTVSet))
    (Utilities|IsValid (.TVMesh (Utilities|Struct|BreakST_TVEntry _array_element))
      (:Is%20Valid
        (Utilities|Map|Add (Variables|Default|GetMeshSizeCache) (.TVMesh (Utilities|Struct|BreakST_TVEntry _array_element)) (* (.boxextent (StaticMesh|GetBounds (.TVMesh (Utilities|Struct|BreakST_TVEntry _array_element)))) 2.0))
        (if (not (< (.Weight (Utilities|Struct|BreakST_TVEntry _array_element)) 0.0))
          (Variables|Default|SetTotalWeight (+ (Variables|Default|GetTotalWeight) (.Weight (Utilities|Struct|BreakST_TVEntry _array_element))))))))
  (if (Variables|TVContent|GetbNormalizeToSlotSize)
    (if (not (Math|Vector|VectorIsZero _targetslotsize))
      (Variables|Default|SetSlotSize _targetslotsize)
      (else
        (Variables|Default|SetSlotSize (.Value (Utilities|Map|GetKeyValueByIndex (Variables|Default|GetMeshSizeCache) 0)))))
    (else
      (bind _values (Utilities|Map|Values (Variables|Default|GetMeshSizeCache)))
      (for _array_element_2 _values
        (Utilities|Array|Add (LocalVariables|GetXArray) (.x _array_element_2))
        (Utilities|Array|Add (LocalVariables|GetYArray) (.y _array_element_2))
        (Utilities|Array|Add (LocalVariables|GetZArray) (.z _array_element_2)))
      (Variables|Default|SetSlotSize (Math|Vector|MakeVector (.MaxValue (Math|Float|MaxOfFloatArray (LocalVariables|GetXArray))) (.MaxValue (Math|Float|MaxOfFloatArray (LocalVariables|GetYArray))) (.MaxValue (Math|Float|MaxOfFloatArray (LocalVariables|GetZArray))))))))

(fn GetColumnCount
  (return (Math|Float|Truncate (/ (Spline|GetSplineLength (Variables|Default|GetSpline_Wall)) (.x (Variables|Default|GetSlotSize))))))

(fn GetColumnBaseTransform
  (params (ColumnIndex :type Integer))
  (return (Spline|GetTransformatDistanceAlongSpline (Variables|Default|GetSpline_Wall) (* (.x (Variables|Default|GetSlotSize)) ColumnIndex) "Local" false)))

(fn GetColumnRows
  (params (ColumnIndex :type Integer) (Distance01 :type Float%20%28double-precision%29))
  (bind _columnoverridemap (Variables|HeightControl|GetColumnOverrideMap))
  (if (Utilities|Map|Contains _columnoverridemap ColumnIndex)
    (LocalVariables|SetRows (.Value (Utilities|Map|Find _columnoverridemap ColumnIndex)))
    (else
      (Utilities|IsValid (Variables|HeightControl|GetHeightProfile)
        (:Is%20Valid
          (LocalVariables|SetRows (Math|Float|Round (Math|Curves|GetFloatValue (Variables|HeightControl|GetHeightProfile) Distance01))))
        (:Is%20Not%20Valid
          (LocalVariables|SetRows (Variables|Default|GetDefaultRows))))))
  (return (LocalVariables|GetRows)))

(fn BiuldPreviewHISM
  (bind _jitterx (Variables|Variation|GetJitterX))
  (bind _randomyaw (Variables|Variation|GetRandomYaw))
  (Variables|Default|SetRandomStream (Math|Random|MakeRandomStream (Variables|TVContent|GetSeed)))
  (Components|InstancedStaticMesh|ClearInstances (Variables|Default|GetHISM_Preview_Default))
  (for _array_element (Variables|Components|GetPreviewHISMs)
    (Components|InstancedStaticMesh|ClearInstances _array_element))
  (CallFunction|EnsurePreviewHISMs)
  (CallFunction|BuildMeshCacheandSlotSize)
  (Variables|Default|SetColumns (CallFunction|GetColumnCount))
  (LocalVariables|SetSplineLenth (Spline|GetSplineLength (Variables|Default|GetSpline_Wall)))
  (LocalVariables|SetColumnStep (.x (Variables|Default|GetSlotSize)))
  ;[0.15 0.15 0.15 0.5] Column loop
  (for _index (range 0 (- (Variables|Default|GetColumns) 1))
    (bind _output_get (LocalVariables|SetDistance (* _index (.x (Variables|Default|GetSlotSize)))))
    (LocalVariables|SetBaseXform (Spline|GetTransformatDistanceAlongSpline (Variables|Default|GetSpline_Wall) _output_get "Local" false))
    (if (> (Variables|Default|GetColumns) 1)
      (LocalVariables|SetDistance01 (/ _index (- (Variables|Default|GetColumns) 1)))
      (else
        (LocalVariables|SetDistance01 0.0)))
    (bind _row (CallFunction|GetColumnRows _index (LocalVariables|GetDistance01)))
    (LocalVariables|SetCurrentZ 0.0)
    ;[0.15 0.15 0.15 0.5] Row loop
    (for _index_2 (range 0 (- _row 1))
      (if (Utilities|Array|IsEmpty (Variables|Components|GetPreviewHISMs))
        (bind _output_get_2 (LocalVariables|SetUpOffset (* (.z (Variables|Default|GetSlotSize)) _index_2)))
        (Components|InstancedStaticMesh|AddInstance (Variables|Default|GetHISM_Preview_Default) (Math|Transform|MakeTransform (+ (Math|Vector|MakeVector 0.0 0.0 _output_get_2) (.location (LocalVariables|GetBaseXform))) (.rotation (LocalVariables|GetBaseXform))) false)
        (else
          (LocalVariables|SetPickValue (Math|Random|RandomFloatinRangefromStream (Variables|Default|GetRandomStream) 0.0 (Variables|Default|GetTotalWeight)))
          (LocalVariables|SetRunningWeight 0.0)
          (bind (_array_element_2 _array_index) (Utilities|Array|ForEachLoopwithBreak (Variables|/Game/Blueprints/PDA_TVSet.PDA_TVSet_C|GetTVEntries (Variables|TVcontent|GetTVSet)) :!label _label)
            (:LoopBody
              (LocalVariables|SetJitterAlong (Math|Random|RandomFloatinRangefromStream (Variables|Default|GetRandomStream) (* _jitterx -1.0) _jitterx))
              (LocalVariables|SetYawOffsetDeg (Math|Random|RandomFloatinRangefromStream (Variables|Default|GetRandomStream) (* _randomyaw -1.0) _randomyaw))
              (LocalVariables|SetRunningWeight (+ (.weight _array_element_2) (LocalVariables|GetRunningWeight)))
              (if (<= (LocalVariables|GetPickValue) (LocalVariables|GetRunningWeight))
                (Components|InstancedStaticMesh|AddInstance (Utilities|Array|Get(acopy) (Variables|Components|GetPreviewHISMs) _array_index) (Math|Transform|MakeTransform (+ (+ (+ (Math|Vector|MakeVector 0.0 0.0 (LocalVariables|GetCurrentZ)) (.location (LocalVariables|GetBaseXform))) (* (Math|Vector|GetRightVector (.rotation (LocalVariables|GetBaseXform))) (* (* (Variables|Layout|GetSpacingY) _index_2) -1.0))) (* (Math|Vector|GetForwardVector (.rotation (LocalVariables|GetBaseXform))) (LocalVariables|GetJitterAlong))) (Math|Rotator|CombineRotators (.rotation (LocalVariables|GetBaseXform)) (Math|Rotator|MakeRotator 0.0 0.0 (LocalVariables|GetYawOffsetDeg)))) false)
                (LocalVariables|SetCurrentZ (+ (.z (.Value (Utilities|Map|Find (Variables|Default|GetMeshSizeCache) (.tvmesh _array_element_2)))) (LocalVariables|GetCurrentZ)))
                (goto _label Break)))))))))

(fn EnsurePreviewHISMs
  (bind _previewhisms (Variables|Components|GetPreviewHISMs))
  (for _array_element (Variables|Components|GetPreviewHISMs)
    (Components|InstancedStaticMesh|ClearInstances _array_element))
  (for _index (range 0 (- (Utilities|Array|Length (Variables|/Game/Blueprints/PDA_TVSet.PDA_TVSet_C|GetTVEntries (Variables|TVcontent|GetTVSet))) 1))
    (if (Utilities|Array|IsValidIndex _previewhisms _index)
      (Utilities|IsValid (Utilities|Array|Get(acopy) _previewhisms _index)
        (:Is%20Valid
          (Components|StaticMesh|SetStaticMesh (Utilities|Array|Get(acopy) _previewhisms _index) (.tvmesh (Utilities|Array|Get(acopy) (Variables|/Game/Blueprints/PDA_TVSet.PDA_TVSet_C|GetTVEntries (Variables|TVcontent|GetTVSet)) _index))))
        (:Is%20Not%20Valid
          (Components|DestroyComponent (Utilities|Array|Get(acopy) _previewhisms _index))
          (bind _returnvalue (AddComponent|AddHierarchicalInstancedStaticMeshComponent false (Math|Transform|MakeTransform "0, 0, 0")))
          (Components|StaticMesh|SetStaticMesh _returnvalue (.tvmesh (Utilities|Array|Get(acopy) (Variables|/Game/Blueprints/PDA_TVSet.PDA_TVSet_C|GetTVEntries (Variables|TVcontent|GetTVSet)) _index)))
          (Utilities|Array|SetArrayElem (Variables|Components|GetPreviewHISMs) _index _returnvalue)))
      (else
        (bind _returnvalue_2 (AddComponent|AddHierarchicalInstancedStaticMeshComponent false (Math|Transform|MakeTransform "0, 0, 0")))
        (Components|StaticMesh|SetStaticMesh _returnvalue_2 (.tvmesh (Utilities|Array|Get(acopy) (Variables|/Game/Blueprints/PDA_TVSet.PDA_TVSet_C|GetTVEntries (Variables|TVcontent|GetTVSet)) _index)))
        (Utilities|Array|Add (Variables|Components|GetPreviewHISMs) _returnvalue_2))))
  (if (> (Utilities|Array|Length (Variables|Components|GetPreviewHISMs)) (Utilities|Array|Length (Variables|/Game/Blueprints/PDA_TVSet.PDA_TVSet_C|GetTVEntries (Variables|TVcontent|GetTVSet))))
    (for _index_2 (range (Utilities|Array|Length (Variables|Components|GetPreviewHISMs)) (- (Utilities|Array|Length (Variables|/Game/Blueprints/PDA_TVSet.PDA_TVSet_C|GetTVEntries (Variables|TVcontent|GetTVSet))) 1))
      (Components|DestroyComponent (Utilities|Array|Get(acopy) (Variables|Components|GetPreviewHISMs) _index_2))
      (Utilities|Array|RemoveIndex (Variables|Components|GetPreviewHISMs) _index_2))))

(fn ClearBaked
  (bind _outactors (Actor|GetAllActorsOfClasswithTag "/Script/Engine.StaticMeshActor" "TV_BAKED"))
  (for _array_element _outactors
    (Actor|DestroyActor _array_element))
  (Variables|Default|SetbBaked false))

(fn BaketoEditable
  (bind _jitterx (Variables|Variation|GetJitterX))
  (bind _randomyaw (Variables|Variation|GetRandomYaw))
  (CallFunction|ClearBaked)
  (CallFunction|BuildMeshCacheandSlotSize)
  (for _array_element (Variables|Components|GetPreviewHISMs)
    (Components|InstancedStaticMesh|ClearInstances _array_element))
  (Variables|Default|SetRandomStream (Math|Random|MakeRandomStream (Variables|TVContent|GetSeed)))
  (LocalVariables|SetSplineLength (Spline|GetSplineLength (Variables|Default|GetSpline_Wall)))
  (LocalVariables|SetColumnStep (.x (Variables|Default|GetSlotSize)))
  (bind _output_get (LocalVariables|SetColumn (CallFunction|GetColumnCount)))
  (if (not (< _output_get 1))
    (for _index (range 0 (- (LocalVariables|GetColumn) 1))
      (bind _output_get_2 (LocalVariables|SetDistance (* _index (.x (Variables|Default|GetSlotSize)))))
      (LocalVariables|SetBase%20Xform (Spline|GetTransformatDistanceAlongSpline (Variables|Default|GetSpline_Wall) _output_get_2 "World" false))
      (if (> (LocalVariables|GetColumn) 1)
        (LocalVariables|SetDistance01 (/ _index (- (LocalVariables|GetColumn) 1)))
        (else
          (LocalVariables|SetDistance01 0.0)))
      (bind _row (CallFunction|GetColumnRows _index (LocalVariables|GetDistance01)))
      (LocalVariables|SetCurrentZ 0.0)
      (for _index_2 (range 0 (- _row 1))
        (LocalVariables|SetPickValue (Math|Random|RandomFloatinRangefromStream (Variables|Default|GetRandomStream) 0.0 (Variables|Default|GetTotalWeight)))
        (LocalVariables|SetRunning%20Weight 0.0)
        (bind _array_element_2 (Utilities|Array|ForEachLoopwithBreak (Variables|/Game/Blueprints/PDA_TVSet.PDA_TVSet_C|GetTVEntries (Variables|TVcontent|GetTVSet)) :!label _label)
          (:LoopBody
            (LocalVariables|SetJitterAlong (Math|Random|RandomFloatinRangefromStream (Variables|Default|GetRandomStream) (* _jitterx -1.0) _jitterx))
            (LocalVariables|SetYaw%20Offset%20Deg (Math|Random|RandomFloatinRangefromStream (Variables|Default|GetRandomStream) (* _randomyaw -1.0) _randomyaw))
            (LocalVariables|SetRunning%20Weight (+ (.weight _array_element_2) (LocalVariables|GetRunning%20Weight)))
            (if (<= (LocalVariables|GetPickValue) (LocalVariables|GetRunning%20Weight))
              (LocalVariables|SetChosenMesh (.tvmesh _array_element_2))
              (bind _returnvalue (Game|SpawnActorfromClass "/Script/Engine.StaticMeshActor" (Math|Transform|MakeTransform (+ (+ (+ (Math|Vector|MakeVector 0.0 0.0 (LocalVariables|GetCurrentZ)) (.location (LocalVariables|GetBase%20Xform))) (* (Math|Vector|GetRightVector (.rotation (LocalVariables|GetBase%20Xform))) (* (* (Variables|Layout|GetSpacingY) _index_2) -1.0))) (* (Math|Vector|GetForwardVector (.rotation (LocalVariables|GetBase%20Xform))) (LocalVariables|GetJitterAlong))) (Math|Rotator|CombineRotators (.rotation (LocalVariables|GetBase%20Xform)) (Math|Rotator|MakeRotator 0.0 0.0 (LocalVariables|GetYaw%20Offset%20Deg)))) "Undefined" "MultiplyWithRoot" 0 0))
              (Class|VCamBlueprintFunctionLibrary|SetActorLabel _returnvalue (Utilities|String|Append (Utilities|String|MakeLiteralString "TV_Mesh_") (Utilities|String|ToString(Integer) (LocalVariables|GetTVNum))))
              (Components|StaticMesh|SetStaticMesh (Variables|/Script/Engine.StaticMeshActor|GetStaticMeshComponent _returnvalue) (LocalVariables|GetChosenMesh))
              (Variables|/Script/Engine.Actor|SetTags _returnvalue (Utilities|Array|MakeArray (Utilities|Name|MakeLiteralName "TV_BAKED")))
              (LocalVariables|SetCurrentZ (+ (.z (.Value (Utilities|Map|Find (Variables|Default|GetMeshSizeCache) (.tvmesh _array_element_2)))) (LocalVariables|GetCurrentZ)))
              (Math|Integer|IncrementInt (LocalVariables|GetTVNum)
                (:%20%20
                  (goto _label Break))))))))
    (Variables|Default|SetbBaked true)))